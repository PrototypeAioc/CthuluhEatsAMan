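; BP_PickUpActor is a world item pickup that gives a set amount of an item class to the third-person character's inventory.
; A sphere overlap registers it in the character's NearbyPickupActor list, and only the first entry shows its prompt widget, handing it on when it leaves.
; OnPickedUp calls AddItem, keeps any leftover amount with refreshed text, or removes itself from the list and destroys itself.
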(event OnComponentBeginOverlap(Sphere)
  (params (OverlappedComponent :type Primitive%20Component%20Object%20Reference) (OtherActor :type Actor%20Object%20Reference) (OtherComp :type Primitive%20Component%20Object%20Reference) (OtherBodyIndex :type Integer) (bFromSweep :type Boolean) (SweepResult :type Hit%20Result%20Structure%20%28by%20ref%29))
  (bind _asthird_person_character (Utilities|Casting|CastToThirdPersonCharacter OtherActor))
  (if (> (Utilities|Array|Length (Variables|/Game/ThirdPersonBP/Blueprints/ThirdPersonCharacter.ThirdPersonCharacter_C|GetNearbyPickupActor _asthird_person_character)) 0)
    (Utilities|Array|Add (Variables|/Game/ThirdPersonBP/Blueprints/ThirdPersonCharacter.ThirdPersonCharacter_C|GetNearbyPickupActor _asthird_person_character) self)
    (else
      (Rendering|SetVisibility (Variables|Default|GetPickupText) true false)
      (Utilities|Array|Add (Variables|/Game/ThirdPersonBP/Blueprints/ThirdPersonCharacter.ThirdPersonCharacter_C|GetNearbyPickupActor _asthird_person_character) self))))

(event OnComponentEndOverlap(Sphere)
  (params (OverlappedComponent :type Primitive%20Component%20Object%20Reference) (OtherActor :type Actor%20Object%20Reference) (OtherComp :type Primitive%20Component%20Object%20Reference) (OtherBodyIndex :type Integer))
  (bind _asthird_person_character (Utilities|Casting|CastToThirdPersonCharacter OtherActor))
  (if (and (Utilities|IsValid (Utilities|Array|Get(acopy) (Variables|/Game/ThirdPersonBP/Blueprints/ThirdPersonCharacter.ThirdPersonCharacter_C|GetNearbyPickupActor _asthird_person_character))) (== (Utilities|Array|Get(acopy) (Variables|/Game/ThirdPersonBP/Blueprints/ThirdPersonCharacter.ThirdPersonCharacter_C|GetNearbyPickupActor _asthird_person_character)) self))
    (Rendering|SetVisibility (Variables|Default|GetPickupText) false false)
    (Utilities|Array|RemoveItem (Variables|/Game/ThirdPersonBP/Blueprints/ThirdPersonCharacter.ThirdPersonCharacter_C|GetNearbyPickupActor _asthird_person_character) self)
    (Utilities|IsValid (Utilities|Array|Get(acopy) (Variables|/Game/ThirdPersonBP/Blueprints/ThirdPersonCharacter.ThirdPersonCharacter_C|GetNearbyPickupActor _asthird_person_character))
      (:Is%20Valid
        (Rendering|SetVisibility (Variables|BP_PickUpActor_C|GetPickupText (Utilities|Array|Get(acopy) (Variables|/Game/ThirdPersonBP/Blueprints/ThirdPersonCharacter.ThirdPersonCharacter_C|GetNearbyPickupActor _asthird_person_character))) true false)))
    (else
      (Utilities|Array|RemoveItem (Variables|/Game/ThirdPersonBP/Blueprints/ThirdPersonCharacter.ThirdPersonCharacter_C|GetNearbyPickupActor _asthird_person_character) self))))

(event Custom|OnPickedUp
  (params (ThirdPersonChar :type Third%20Person%20Character%20Object%20Reference))
  (bind _nearbypickupactor (Variables|/Game/ThirdPersonBP/Blueprints/ThirdPersonCharacter.ThirdPersonCharacter_C|GetNearbyPickupActor ThirdPersonChar))
  (bind _inventoryref (Variables|/Game/ThirdPersonBP/Blueprints/ThirdPersonCharacter.ThirdPersonCharacter_C|GetInventoryRef ThirdPersonChar))
  (bind _item (Utilities|Array|Get(acopy) _nearbypickupactor))
  (Utilities|IsValid _inventoryref
    (:Is%20Valid
      (bind (_success_ _rest) (Default|AddItem _inventoryref (Variables|Default|GetItemToAdd) (Variables|Default|GetAmount)))
      (if _success_
        (if (> _rest 0)
          (Variables|Default|SetAmount _rest)
          (CallFunction|UpdateText)
          (else
            (Utilities|Array|RemoveItem _nearbypickupactor self)
            (Utilities|IsValid _item
              (:Is%20Valid
                (Rendering|SetVisibility (Variables|BP_PickUpActor_C|GetPickupText _item) true false)
                (Actor|DestroyActor))
              (:Is%20Not%20Valid
                (Actor|DestroyActor)))))))))

(event EventBeginPlay
  (CallFunction|UpdateText))

(event Collision|EventActorBeginOverlap
  (params (OtherActor :type Actor%20Object%20Reference)))

(event EventTick
  (params (DeltaSeconds :type Float%20%28single-precision%29)))

(fn ConstructionScript)

(fn UpdateText
  (bind _aspick_up_text (Utilities|Casting|CastToPickUpText (UserInterface|GetUserWidgetObject (Variables|Default|GetPickupText)))
    (:then
      (Rendering|Components|TextRender|SetText (Variables|/Game/Inventory_System/Widgets/PickUpText.PickUpText_C|GetNameText _aspick_up_text) (Utilities|Text|FormatText "{Name} {Amount}" (.Name (Utilities|Struct|BreakS_ItemInfo (.OneItemInfo (Utilities|GetClassDefaults (Variables|Default|GetItemToAdd))))) (Variables|Default|GetAmount))))
    (:CastFailed
      _))
  (return))